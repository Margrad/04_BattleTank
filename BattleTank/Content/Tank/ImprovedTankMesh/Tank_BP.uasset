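; Player tank Blueprint that wires input to track-based driving, camera aiming and firing.
; On BeginPlay it hands the turret and barrel components to the tank and initialises TankMovement with both tracks.
; Throttle axes drive each track directly, while forward and right axes send movement intents through TankMovement.
; Aim axes yaw an azimuth gimbal and pitch the spring arm separately, and the Fire action calls Fire.
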(event `self.ReceiveBeginPlay`
  (`self.SetTurretReference` (`self.TankTurret`))
  (`self.SetBarrelReference` (`self.TankBarrel1`))
  (`TankMovementComponent.Initialise` (`self.TankMovement`) (`self.LeftTrack`) (`self.RightTrack`)))

(event `InputAxis|LeftThrottle`
  (params (AxisValue :type "Float (single-precision)"))
  ;[1 1 1] Keyboard Movement Controls
  (`TankTrack.SetThrottle` (`self.LeftTrack`) AxisValue))

(event `InputAxis|AimElevation`
  (params (AxisValue :type "Float (single-precision)"))
  ;[1 1 1] Mouse Controls
  (`SceneComponent.K2_AddLocalRotation` (`self.SpringArm_0`) (`KismetMathLibrary.MakeRotator` 0.0 AxisValue) false false))

(event `InputAxis|RightThrottle`
  (params (AxisValue :type "Float (single-precision)"))
  ;[1 1 1] Keyboard Movement Controls
  (`TankTrack.SetThrottle` (`self.RightTrack`) AxisValue))

(event `InputAxis|AimAzimuth`
  (params (AxisValue :type "Float (single-precision)"))
  ;[1 1 1] Mouse Controls
  (`SceneComponent.K2_AddLocalRotation` (`self.AzimouthGimball`) (`KismetMathLibrary.MakeRotator` 0.0 0.0 AxisValue) false false))

(event `InputAxis|FowardMovement`
  (params (AxisValue :type "Float (single-precision)"))
  ;[1 1 1] Keyboard Movement Controls
  (`TankMovementComponent.IntendMoveForward` (`self.TankMovement`) AxisValue))

(event `InputAction|Fire`
  (params (Key :type "Key Structure"))
  ;[1 1 1] Mouse Controls
  (:`Pressed`
    (`self.Fire`)))

(event `InputAxis|RightMovement`
  (params (AxisValue :type "Float (single-precision)"))
  ;[1 1 1] Keyboard Movement Controls
  (`TankMovementComponent.IntendTurnRight` (`self.TankMovement`) AxisValue))

(fn `UserConstructionScript`)