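; Player-drivable tank pawn Blueprint that wires input and components to the movement, aiming and health bar systems.
; On BeginPlay it passes barrel and turret to Aiming, both tracks to TankMovement, and itself to the HealthBar widget.
; Axis inputs send move and turn intents to TankMovement and rotate the camera for pitch and an azimuth gimbal for yaw.
; The Fire action calls Aiming.Fire.
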(event `self.ReceiveBeginPlay`
  (`AimingComponent.Initialise` (`self.Aiming`) (`self.TankBarrel`) (`self.TankTurret`))
  (`TankMovementComponent.Initialise` (`self.TankMovement`) (`self.LeftTrack`) (`self.RightTrack`))
  (bind _ashealth_bar (cast `/Game/UI/HealthBar` (`WidgetComponent.GetUserWidgetObject` (`self.Widget`))))
  (set `/Game/UI/HealthBar.ThisTank` self _ashealth_bar))

(event `InputAxis|FowardMovement`
  (params (AxisValue :type "Float (single-precision)"))
  (`TankMovementComponent.IntendMoveForward` (`self.TankMovement`) AxisValue))

(event `InputAxis|AimElevation`
  (params (AxisValue :type "Float (single-precision)"))
  (`SceneComponent.K2_AddLocalRotation` (`self.Camera`) (`KismetMathLibrary.MakeRotator` 0.0 AxisValue) false false))

(event `InputAxis|RightMovement`
  (params (AxisValue :type "Float (single-precision)"))
  (`TankMovementComponent.IntendTurnRight` (`self.TankMovement`) AxisValue))

(event `InputAxis|AimAzimuth`
  (params (AxisValue :type "Float (single-precision)"))
  (`SceneComponent.K2_AddLocalRotation` (`self.AzimoutGimball`) (`KismetMathLibrary.MakeRotator` 0.0 0.0 AxisValue) false false))

(event `InputAction|Fire`
  (params (Key :type "Key Structure"))
  (:`Pressed`
    (`AimingComponent.Fire` (`self.Aiming`))))

(fn `UserConstructionScript`)